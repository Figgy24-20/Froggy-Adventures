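; Camera manager actor that follows the player's BP_Froggy character along X and Z within level-specific bounds.
; On BeginPlay it reads the current level from GI_main and picks the X and Z max limits from size presets.
; Each Tick, UpdateCameraPos clamps the frog's position, offset downward in Z, and eases toward it with VInterpTo.
; The Z limit names run inverted: ZLimitMax is the lower bound and ZLimitMin the upper.
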(event Collision|EventActorBeginOverlap
  (params (OtherActor :type Actor%20Object%20Reference)))

(event EventTick
  (params (DeltaSeconds :type Float%20%28single-precision%29))
  (CallFunction|UpdateCameraPos))

(event EventBeginPlay
  ;[1 1 1 1 40] Update Limits
  (bind _asgi_main (Utilities|Casting|CastToGI_main (Game|GetGameInstance)))
  (if (Math|Boolean|ORBoolean (== (Variables|/Game/blueprints/Utilities/GI_main.GI_main_C|GetLevel _asgi_main) (Variables|Default|GetLevel_3_1)) (== (Variables|/Game/blueprints/Utilities/GI_main.GI_main_C|GetLevel _asgi_main) (Variables|Default|GetLevel_3_2)) (== (Variables|/Game/blueprints/Utilities/GI_main.GI_main_C|GetLevel _asgi_main) (Variables|Default|GetLevel_3_3)) (== (Variables|/Game/blueprints/Utilities/GI_main.GI_main_C|GetLevel _asgi_main) (Variables|Default|GetLevel_3_4)))
    (Variables|Default|SetxLimitMax (Variables|Default|GetxLimitMax_Big))
    (Variables|Default|SetzLimitMax (Variables|Default|GetzLimitMax_small))
    (elif (== (Variables|/Game/blueprints/Utilities/GI_main.GI_main_C|GetLevel _asgi_main) (Variables|Default|GetLevel_5))
      (Variables|Default|SetxLimitMax (Variables|Default|GetxLimitMax_Huge))
      (Variables|Default|SetzLimitMax (Variables|Default|GetzLimitMax_big))
      (else
        (Variables|Default|SetxLimitMax (Variables|Default|GetxLimitMax_Small))
        (Variables|Default|SetzLimitMax (Variables|Default|GetzLimitMax_small))))))

(fn ConstructionScript)

(fn UpdateCameraPos
  (bind _xlimitmin (Variables|Default|GetxLimitMin))
  (bind _xlimitmax (Variables|Default|GetxLimitMax))
  (bind _zlimitmax (Variables|Default|GetzLimitMax))
  (bind _zlimitmin (Variables|Default|GetzLimitMin))
  (bind _asbp_froggy (Utilities|Casting|CastToBP_Froggy (Game|GetPlayerCharacter 0)))
  (if true
    (Transformation|SetActorLocation (Math|Vector|MakeVector (.x (Math|Interpolation|VInterpTo (Transformation|GetActorLocation) (Math|Vector|MakeVector (Math|Float|SelectFloat _xlimitmax (Math|Float|SelectFloat _xlimitmin (.x (Transformation|GetActorLocation _asbp_froggy)) (< (.x (Transformation|GetActorLocation _asbp_froggy)) _xlimitmin)) (> (Math|Float|SelectFloat _xlimitmin (.x (Transformation|GetActorLocation _asbp_froggy)) (< (.x (Transformation|GetActorLocation _asbp_froggy)) _xlimitmin)) _xlimitmax)) 0.0 (Math|Float|SelectFloat _zlimitmin (Math|Float|SelectFloat _zlimitmax (- (.z (Transformation|GetActorLocation _asbp_froggy)) 1e+02) (< (- (.z (Transformation|GetActorLocation _asbp_froggy)) 1e+02) _zlimitmax)) (> (Math|Float|SelectFloat _zlimitmax (- (.z (Transformation|GetActorLocation _asbp_froggy)) 1e+02) (< (- (.z (Transformation|GetActorLocation _asbp_froggy)) 1e+02) _zlimitmax)) _zlimitmin))) (Utilities|Time|GetWorldDeltaSeconds) 5.0)) 0.0 (.z (Math|Interpolation|VInterpTo (Transformation|GetActorLocation) (Math|Vector|MakeVector (Math|Float|SelectFloat _xlimitmax (Math|Float|SelectFloat _xlimitmin (.x (Transformation|GetActorLocation _asbp_froggy)) (< (.x (Transformation|GetActorLocation _asbp_froggy)) _xlimitmin)) (> (Math|Float|SelectFloat _xlimitmin (.x (Transformation|GetActorLocation _asbp_froggy)) (< (.x (Transformation|GetActorLocation _asbp_froggy)) _xlimitmin)) _xlimitmax)) 0.0 (Math|Float|SelectFloat _zlimitmin (Math|Float|SelectFloat _zlimitmax (- (.z (Transformation|GetActorLocation _asbp_froggy)) 1e+02) (< (- (.z (Transformation|GetActorLocation _asbp_froggy)) 1e+02) _zlimitmax)) (> (Math|Float|SelectFloat _zlimitmax (- (.z (Transformation|GetActorLocation _asbp_froggy)) 1e+02) (< (- (.z (Transformation|GetActorLocation _asbp_froggy)) 1e+02) _zlimitmax)) _zlimitmin))) (Utilities|Time|GetWorldDeltaSeconds) 5.0))) false false)))