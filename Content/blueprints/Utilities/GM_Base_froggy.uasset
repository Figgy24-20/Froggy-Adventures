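; Base game mode blueprint, with hooks for loading and saving at the start and end of play.
; BeginPlay calls LoadGame, which only casts and caches the GI_main game instance.
; EndPlay calls SaveGame, which is currently empty.
; High-score persistence through SG_HighScore_0 save slots remains in both functions as disconnected nodes, so it never runs.
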(event EventBeginPlay
  (CallFunction|LoadGame))

(event EventTick
  (params (DeltaSeconds :type Float%20%28single-precision%29)))

(event EventEndPlay
  (params (EndPlayReason :type EEndPlayReason%20Enum :default "Destroyed"))
  (CallFunction|SaveGame))

(fn ConstructionScript)

(fn LoadGame
  (bind _asgi_main (Utilities|Casting|CastToGI_main (Game|GetGameInstance)))
  (Variables|Default|SetAs%20GI%20Main _asgi_main))

(fn SaveGame)