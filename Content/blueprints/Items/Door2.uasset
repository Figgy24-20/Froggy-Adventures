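; Paper2D door actor that either shines or closes and loads level 1_1 when something overlaps its box.
; The overlap event reads the Door11 flag from BP_MainGameInstance and, if set, only switches the flipbook to the shine animation.
; Otherwise, a chain of delays plays the closing flipbook, swaps to the static closed one, then opens the level.
; The overlapping actor is not filtered.
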(event OnComponentBeginOverlap(Box)
  (params (OverlappedComponent :type Primitive%20Component%20Object%20Reference) (OtherActor :type Actor%20Object%20Reference) (OtherComp :type Primitive%20Component%20Object%20Reference) (OtherBodyIndex :type Integer) (bFromSweep :type Boolean) (SweepResult :type Hit%20Result%20Structure%20%28by%20ref%29))
  (bind _asbp_main_game_instance (Utilities|Casting|CastToBP_MainGameInstance (Game|GetGameInstance)))
  (if (Variables|/Game/blueprints/BP_MainGameInstance.BP_MainGameInstance_C|GetDoor1_1 _asbp_main_game_instance)
    (Sprite|SetFlipbook (Variables|Default|GetPaperFlipbook) "/Game/Assets/Items/Door/Door_Shine/FP_Door_Shine.FP_Door_Shine")
    (else
      (Utilities|FlowControl|Delay 1.0)
      (Sprite|SetFlipbook (Variables|Default|GetPaperFlipbook) "/Game/Assets/Items/Door/Door_Close/FP_Door_Close.FP_Door_Close")
      (Utilities|FlowControl|Delay 1.0)
      (Sprite|SetFlipbook (Variables|Default|GetPaperFlipbook) "/Game/Assets/Items/Door/Door_Close/Door_Close_Static.Door_Close_Static")
      (Utilities|FlowControl|Delay 0.2)
      (Game|OpenLevel(byObjectReference) "/Game/Maps/1_1_level.1_1_level"))))

(event EventBeginPlay)

(event Collision|EventActorBeginOverlap
  (params (OtherActor :type Actor%20Object%20Reference)))

(event EventTick
  (params (DeltaSeconds :type Float%20%28single-precision%29)))

(fn ConstructionScript)