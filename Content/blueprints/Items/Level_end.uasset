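; Level-end trigger actor that finishes the current level when the frog player (BP_Froggy) enters its Box.
; On overlap it plays a loud 2D splash sound, waits two seconds, then sets the Door11 flag on BP_MainGameInstance and opens the level referenced by Levels.
; The flag lives on the game instance, so it persists across the level change.
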(event OnComponentBeginOverlap(Box)
  (params (OverlappedComponent :type Primitive%20Component%20Object%20Reference) (OtherActor :type Actor%20Object%20Reference) (OtherComp :type Primitive%20Component%20Object%20Reference) (OtherBodyIndex :type Integer) (bFromSweep :type Boolean) (SweepResult :type Hit%20Result%20Structure%20%28by%20ref%29))
  (Utilities|Casting|CastToBP_Froggy OtherActor)
  (Audio|PlaySound2D "/Game/Assets/SFX/Splash.Splash" 3.0 1.0 0.0 0 0)
  (Utilities|FlowControl|Delay 2.0)
  (Utilities|FlowControl|Sequence
    (:then_0
      (bind _asbp_main_game_instance (Utilities|Casting|CastToBP_MainGameInstance (Game|GetGameInstance)))
      (Variables|/Game/blueprints/BP_MainGameInstance.BP_MainGameInstance_C|SetDoor1_1 _asbp_main_game_instance true))
    (:then_1
      (Game|OpenLevel(byObjectReference) "/Game/Maps/Levels.Levels"))))

(event EventBeginPlay
  (|CallParentFunction) ; This node is disabled and will not be called.\nDrag off pins to build functionality.
)

(event Collision|EventActorBeginOverlap
  (params (OtherActor :type Actor%20Object%20Reference))
  (|CallParentFunction OtherActor) ; This node is disabled and will not be called.\nDrag off pins to build functionality.
)

(event EventTick
  (params (DeltaSeconds :type Float%20%28single-precision%29))
  (|CallParentFunction DeltaSeconds) ; This node is disabled and will not be called.\nDrag off pins to build functionality.
)

(fn ConstructionScript
  (|CallParentFunction))