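; Heart_BP is a heart pickup that grants an extra life when BP_Froggy overlaps its box.
; On overlap it plays the Heart sound, scaled by the SFX volume stored in the GI_main game instance, and increments that instance's LifeCount.
; After a brief delay the actor destroys itself.
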(event OnComponentBeginOverlap(Box)
  (params (OverlappedComponent :type Primitive%20Component%20Object%20Reference) (OtherActor :type Actor%20Object%20Reference) (OtherComp :type Primitive%20Component%20Object%20Reference) (OtherBodyIndex :type Integer) (bFromSweep :type Boolean) (SweepResult :type Hit%20Result%20Structure%20%28by%20ref%29))
  (Utilities|Casting|CastToBP_Froggy OtherActor)
  (bind _asgi_main (Utilities|Casting|CastToGI_main (Game|GetGameInstance)))
  (Audio|PlaySound2D "/Game/Assets/SFX/Heart.Heart" (* (Variables|/Game/blueprints/Utilities/GI_main.GI_main_C|GetVolumeSFX _asgi_main) 2.0) 1.0 0.0 0 0)
  (bind _asgi_main_2 (Utilities|Casting|CastToGI_main (Game|GetGameInstance)))
  (Math|Integer|IncrementInt (Variables|/Game/blueprints/Utilities/GI_main.GI_main_C|GetLifeCount _asgi_main_2)
    (:%20%20
      (Utilities|FlowControl|Delay 0.1)
      (Actor|DestroyActor))))

(event EventBeginPlay
  (|CallParentFunction) ; This node is disabled and will not be called.\nDrag off pins to build functionality.
)

(event Collision|EventActorBeginOverlap
  (params (OtherActor :type Actor%20Object%20Reference))
  (|CallParentFunction OtherActor) ; This node is disabled and will not be called.\nDrag off pins to build functionality.
)

(event EventTick
  (params (DeltaSeconds :type Float%20%28single-precision%29))
  (|CallParentFunction DeltaSeconds) ; This node is disabled and will not be called.\nDrag off pins to build functionality.
)

(fn ConstructionScript
  (|CallParentFunction))