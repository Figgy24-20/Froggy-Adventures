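; BP_Waxworm1 is an enemy character that crawls back and forth along the X axis.
; Each tick it moves only if the player's BP_Froggy is past a point a short distance behind it on X, with no upper limit.
; While active, it turns to match its X velocity and destroys itself if it falls too far.
; Any Hit event flips CrickDirection, reversing its movement.
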(event Custom|update%20direction
  (Utilities|IsValid (Pawn|GetController)
    (:Is%20Valid
      (Math|Float|CompareFloat (.X (Class|KismetMathLibrary|BreakVector3f (Variables|/Script/Engine.MovementComponent|GetVelocity (Variables|Character|GetCharacterMovement)))) 0.0
        (:>
          (Transformation|SetActorRotation "0, 0, 0"))
        (:<
          (Transformation|SetActorRotation "0.000000,180.000000,0.000000"))))))

(event Collision|EventHit
  (params (MyComp :type Primitive%20Component%20Object%20Reference) (Other :type Actor%20Object%20Reference) (OtherComp :type Primitive%20Component%20Object%20Reference) (bSelfMoved :type Boolean) (HitLocation :type Vector :default "0, 0, 0") (HitNormal :type Vector :default "0, 0, 0") (NormalImpulse :type Vector :default "0, 0, 0") (Hit :type Hit%20Result%20Structure%20%28by%20ref%29))
  (Variables|Default|SetCrickDirection (* (Variables|Default|GetCrickDirection) -1.0)))

(event EventTick
  (params (DeltaSeconds :type Float%20%28single-precision%29))
  ;[1 1 1] Is Frog Close?
  (bind _asbp_froggy (Utilities|Casting|CastToBP_Froggy (Game|GetPlayerCharacter 0)))
  (if (> (.x (Transformation|GetActorLocation _asbp_froggy)) (- (.x (Transformation|GetActorLocation)) 4.2e+02))
    (CallFunction|UpdateDirection)
    (Pawn|Input|AddMovementInput "0.050000,0.000000,0.000000" (Variables|Default|GetCrickDirection) false)
    (if (< (.z (Transformation|GetActorLocation)) -2e+03)
      (Actor|DestroyActor))))

(event Collision|EventActorBeginOverlap
  (params (OtherActor :type Actor%20Object%20Reference)))

(fn ConstructionScript)