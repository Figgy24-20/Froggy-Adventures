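; BP_Hornworm is a Paper2D enemy that walks along the X axis and turns around whenever it hits something.
; Tick moves it only once the frog player's X passes 400 units before its own, destroying it if it falls too low.
; The sign of CricketSpeed sets direction and facing, and Hit inverts it.
; Timer-based sprite flicker helpers exist, but their only calls sit in unconnected nodes.
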(event Collision|EventActorBeginOverlap
  (params (OtherActor :type Actor%20Object%20Reference)))

(event Collision|EventHit
  (params (MyComp :type Primitive%20Component%20Object%20Reference) (Other :type Actor%20Object%20Reference) (OtherComp :type Primitive%20Component%20Object%20Reference) (bSelfMoved :type Boolean) (HitLocation :type Vector :default "0, 0, 0") (HitNormal :type Vector :default "0, 0, 0") (NormalImpulse :type Vector :default "0, 0, 0") (Hit :type Hit%20Result%20Structure%20%28by%20ref%29))
  ;[1 1 1] Movement
  (bind _output_get (Variables|Default|SetCricket%20Speed (* (Variables|Default|GetCricket%20Speed) -1.0))))

(event EventTick
  (params (DeltaSeconds :type Float%20%28single-precision%29))
  ;[1 1 1] Is Frog Close?
  (bind _asbp_froggy (Utilities|Casting|CastToBP_Froggy (Game|GetPlayerCharacter 0)))
  (if (> (.x (Transformation|GetActorLocation _asbp_froggy)) (- (.x (Transformation|GetActorLocation)) 4e+02))
    ;[1 1 1] Movement
    (Pawn|Input|AddMovementInput (Math|Vector|MakeVector -5e+03 0.0 0.0) (* (stale Collision|EventHit _output_get) 1e+01) false)
    (Transformation|SetActorRotation (Math|Rotator|MakeRotator 0.0 0.0 (+ (* (* (Variables|Default|GetCricket%20Speed) -1.0) (+ 0.0 9e+01)) 9e+01)))
    ;[1 1 1] Despawn if off screen
    (if (< (.z (Transformation|GetActorLocation)) -805.0)
      (Actor|DestroyActor))))

(fn ConstructionScript)

(fn ToggleSpriteFlicker
  (Rendering|SetVisibility (Variables|Default|GetPaperFlipbook) (not (Variables|/Script/Engine.SceneComponent|GetbVisible (Variables|Default|GetPaperFlipbook))) false))

(fn StartSpriteFlicker
  (bind _returnvalue (Utilities|Time|SetTimerbyEvent (EventDispatchers|CreateEvent :!event ToggleSpriteFlicker) (Variables|Default|GetFlickerInterval) true))
  (Variables|Default|SetSpriteFlickerHandle _returnvalue))

(fn StopSpriteFlicker
  (Utilities|Time|ClearandInvalidateTimerbyHandle (Variables|Default|GetSpriteFlickerHandle))
  (Rendering|SetVisibility (Variables|Default|GetPaperFlipbook) true false))

(fn BeginMotion)