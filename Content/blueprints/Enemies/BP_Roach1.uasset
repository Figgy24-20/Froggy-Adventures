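; BP_Roach1 is a flipbook-sprite roach enemy that walks along X and reverses direction whenever it hits something.
; It only updates once BP_Froggy's X passes the roach's X minus EnemySpawnDistance, turning to face its velocity and destroying itself below a height limit.
; When RoachDead is set, it stops, shows a dead flipbook and disables collision, then revives after a delay, always heading +X.
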(event Custom|update%20direction
  (Utilities|IsValid (Pawn|GetController)
    (:Is%20Valid
      (Math|Float|CompareFloat (.X (Class|KismetMathLibrary|BreakVector3f (Variables|/Script/Engine.MovementComponent|GetVelocity (Variables|Character|GetCharacterMovement)))) 0.0
        (:>
          (Transformation|SetActorRotation "0, 0, 0"))
        (:<
          (Transformation|SetActorRotation "0.000000,180.000000,0.000000"))))))

(event Collision|EventHit
  (params (MyComp :type Primitive%20Component%20Object%20Reference) (Other :type Actor%20Object%20Reference) (OtherComp :type Primitive%20Component%20Object%20Reference) (bSelfMoved :type Boolean) (HitLocation :type Vector :default "0, 0, 0") (HitNormal :type Vector :default "0, 0, 0") (NormalImpulse :type Vector :default "0, 0, 0") (Hit :type Hit%20Result%20Structure%20%28by%20ref%29))
  (Variables|Default|SetCrickDirection (* (Variables|Default|GetCrickDirection) -1.0)))

(event EventTick
  (params (DeltaSeconds :type Float%20%28single-precision%29))
  ;[1 1 1] Is Frog Close?
  (bind _asbp_froggy (Utilities|Casting|CastToBP_Froggy (Game|GetPlayerCharacter 0)))
  (if (> (.x (Transformation|GetActorLocation _asbp_froggy)) (- (.x (Transformation|GetActorLocation)) (Variables|/Game/blueprints/Froggy/BP_Froggy.BP_Froggy_C|GetEnemy%20spawn%20distance _asbp_froggy)))
    (CallFunction|UpdateDirection)
    (Pawn|Input|AddMovementInput "0.100000,0.000000,0.000000" (Variables|Default|GetCrickDirection) false)
    (Utilities|FlowControl|Sequence
      (:then_0
        (if (< (.z (Transformation|GetActorLocation)) -2e+03)
          (Actor|DestroyActor)))
      (:then_1
        (if (Variables|Default|GetRoachDead)
          (Sprite|SetFlipbook (Variables|Default|GetSprite) "/Game/Assets/Enemies/roach/Roach-dead_Flipbook.Roach-dead_Flipbook")
          (Variables|Default|SetCrickDirection 0.0)
          (Collision|SetCollisionEnabled (Variables|Default|GetCapsuleComponent) "NoCollision")
          (Utilities|FlowControl|Delay 3.0)
          (Variables|Default|SetCrickDirection 1.0)
          (Sprite|SetFlipbook (Variables|Default|GetSprite) "/Game/Assets/Enemies/roach/roach_book.roach_book")
          (Variables|Default|SetRoachDead false)
          (Collision|SetCollisionEnabled (Variables|Default|GetCapsuleComponent) "QueryAndPhysics"))))))

(event Collision|EventActorBeginOverlap
  (params (OtherActor :type Actor%20Object%20Reference)))

(fn ConstructionScript)