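; Camera manager actor that follows the player's BP_Froggy character on the X and Z axes, as in a side-on view.
; Every Tick, UpdateCameraPos reads Froggy's location and clamps X and Z to min/max limit variables using nested float selects.
; It eases its own location toward that point with VInterpTo, setting only X and Z and leaving the Y input unwired.
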(event EventBeginPlay)

(event Collision|EventActorBeginOverlap
  (params (OtherActor :type Actor%20Object%20Reference)))

(event EventTick
  (params (DeltaSeconds :type Float%20%28single-precision%29))
  (CallFunction|UpdateCameraPos))

(fn ConstructionScript)

(fn UpdateCameraPos
  (bind _xlimitmin (Variables|Default|GetxLimitMin))
  (bind _zlimitmin (Variables|Default|GetzLimitMin))
  (bind _zlimitmax (Variables|Default|GetzLimitMax))
  (bind _xlimitmax (Variables|Default|GetxLimitMax))
  (bind _asbp_froggy (Utilities|Casting|CastToBP_Froggy (Game|GetPlayerCharacter 0)))
  (if true
    (Transformation|SetActorLocation (Math|Vector|MakeVector (.x (Math|Interpolation|VInterpTo (Transformation|GetActorLocation) (Math|Vector|MakeVector (Math|Float|SelectFloat _xlimitmax (Math|Float|SelectFloat _xlimitmin (.x (Transformation|GetActorLocation _asbp_froggy)) (< (.x (Transformation|GetActorLocation _asbp_froggy)) _xlimitmin)) (> (Math|Float|SelectFloat _xlimitmin (.x (Transformation|GetActorLocation _asbp_froggy)) (< (.x (Transformation|GetActorLocation _asbp_froggy)) _xlimitmin)) _xlimitmax)) 0.0 (Math|Float|SelectFloat _zlimitmax (Math|Float|SelectFloat _zlimitmin (.z (Transformation|GetActorLocation _asbp_froggy)) (< (.z (Transformation|GetActorLocation _asbp_froggy)) _zlimitmin)) (> (Math|Float|SelectFloat _zlimitmin (.z (Transformation|GetActorLocation _asbp_froggy)) (< (.z (Transformation|GetActorLocation _asbp_froggy)) _zlimitmin)) _zlimitmax))) (Utilities|Time|GetWorldDeltaSeconds) 5.0)) 0.0 (.z (Math|Interpolation|VInterpTo (Transformation|GetActorLocation) (Math|Vector|MakeVector (Math|Float|SelectFloat _xlimitmax (Math|Float|SelectFloat _xlimitmin (.x (Transformation|GetActorLocation _asbp_froggy)) (< (.x (Transformation|GetActorLocation _asbp_froggy)) _xlimitmin)) (> (Math|Float|SelectFloat _xlimitmin (.x (Transformation|GetActorLocation _asbp_froggy)) (< (.x (Transformation|GetActorLocation _asbp_froggy)) _xlimitmin)) _xlimitmax)) 0.0 (Math|Float|SelectFloat _zlimitmax (Math|Float|SelectFloat _zlimitmin (.z (Transformation|GetActorLocation _asbp_froggy)) (< (.z (Transformation|GetActorLocation _asbp_froggy)) _zlimitmin)) (> (Math|Float|SelectFloat _zlimitmin (.z (Transformation|GetActorLocation _asbp_froggy)) (< (.z (Transformation|GetActorLocation _asbp_froggy)) _zlimitmin)) _zlimitmax))) (Utilities|Time|GetWorldDeltaSeconds) 5.0))) false false)))